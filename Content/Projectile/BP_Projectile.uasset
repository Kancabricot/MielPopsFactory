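; BP_Projectile is a projectile actor that flies until it hits something other than the player, then destroys itself.
; The construction script feeds its InitialSpeed and Gravity variables into the ProjectileMovement component.
; On a collision hit it ignores BP_Player, otherwise stops movement, disables collision and deactivates the trail before destruction.
; A node setting a User.ProjSpeed effect parameter from speed and density is disconnected and never runs.
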(event OnComponentHit(Collision)
  (params (HitComponent :type Primitive%20Component%20Object%20Reference) (OtherActor :type Actor%20Object%20Reference) (OtherComp :type Primitive%20Component%20Object%20Reference) (NormalImpulse :type Vector :default "0, 0, 0") (Hit :type Hit%20Result%20Structure%20%28by%20ref%29))
  (Utilities|Casting|CastToBP_Player OtherActor ; Si c'est le joueur ne fait rien
    (:CastFailed
      (Components|Movement|StopMovementImmediately (Variables|Default|GetProjectileMovement))
      (Collision|SetCollisionEnabled (Variables|Default|GetCollision) "NoCollision")
      (Components|Activation|Deactivate (Variables|Default|GetTrail))
      (Actor|DestroyActor))))

(fn ConstructionScript
  (Variables|/Script/Engine.ProjectileMovementComponent|SetInitialSpeed (Variables|Default|GetProjectileMovement) (Variables|Default|GetInitial%20Speed))
  (Variables|/Script/Engine.ProjectileMovementComponent|SetProjectileGravityScale (Variables|Default|GetProjectileMovement) (Math|Conversions|ToFloat(Boolean) (Variables|Default|GetGravity))))