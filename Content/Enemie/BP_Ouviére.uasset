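; BP_Ouviére is a bee enemy that chases the player and respawns them on contact.
; ProjectileMovement homes on the player; a looping timer checks range, stops the bee, predicts a straight path, then dashes along it.
; Reaching the predicted endpoint or bouncing restores homing and facing.
; A BP_Projectile hit launches the bee along the shot, plays a stuck-death animation and disables it; overlapping Map1 quits the game.
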(event OnComponentBeginOverlap(AbeilleCollision)
  (params (OverlappedComponent :type Primitive%20Component%20Object%20Reference) (OtherActor :type Actor%20Object%20Reference) (OtherComp :type Primitive%20Component%20Object%20Reference) (OtherBodyIndex :type Integer) (bFromSweep :type Boolean) (SweepResult :type Hit%20Result%20Structure%20%28by%20ref%29))
  (bind _projectilemovement (Variables|Default|GetProjectileMovement))
  (if (== OtherComp "/Game/GameArt/Map1.Map1")
    (Game|QuitGame 0 "Quit" false)
    (else
      (bind _asbp_projectile (Utilities|Casting|CastToBP_Projectile OtherActor))
      (Utilities|IsValid _asbp_projectile
        (:Is%20Valid
          (Audio|PlaySoundatLocation "/Game/SFX/C_Impact_Gun.C_Impact_Gun" (Transformation|GetActorLocation) "0, 0, 0" 0.6 1.0 0.0 0 0 0 0)
          (Variables|/Script/Engine.ProjectileMovementComponent|SetbIsHomingProjectile _projectilemovement false)
          (Variables|/Script/Engine.ProjectileMovementComponent|SetbShouldBounce _projectilemovement false)
          (Variables|/Script/Engine.ProjectileMovementComponent|SetMaxSpeed _projectilemovement 3e+03)
          (Variables|/Script/Engine.MovementComponent|SetVelocity _projectilemovement (* (Math|Vector|GetForwardVector (Variables|/Game/Projectile/BP_Projectile.BP_Projectile_C|GetArrow _asbp_projectile)) 3e+03))
          (bind _returnvalue (AddComponent|AddStaticMeshComponent false))
          (Transformation|AttachComponentToComponent _returnvalue (Variables|Default|GetSphere) "None" "KeepRelative" "KeepRelative" "KeepRelative" true)
          (Components|Animation|PlayAnimation (Variables|Default|GetSkeletalMesh) "/Game/GameArt/Chara/A_Bee_DeathStuck_1_Anim.A_Bee_DeathStuck_1_Anim" true)
          (Variables|Default|SetOff true)
          (Variables|Default|SetWatchPlayer false))))))

(event OnComponentBeginOverlap(Sphere)
  (params (OverlappedComponent :type Primitive%20Component%20Object%20Reference) (OtherActor :type Actor%20Object%20Reference) (OtherComp :type Primitive%20Component%20Object%20Reference) (OtherBodyIndex :type Integer) (bFromSweep :type Boolean) (SweepResult :type Hit%20Result%20Structure%20%28by%20ref%29)))

(event OnComponentHit(AbeilleCollision)
  (params (HitComponent :type Primitive%20Component%20Object%20Reference) (OtherActor :type Actor%20Object%20Reference) (OtherComp :type Primitive%20Component%20Object%20Reference) (NormalImpulse :type Vector :default "0, 0, 0") (Hit :type Hit%20Result%20Structure%20%28by%20ref%29))
  (Development|PrintString "Hit")
  (bind _asbp_player (Utilities|Casting|CastToBP_Player OtherActor))
  (Default|Respaw, _asbp_player)
  (Audio|PlaySoundatLocation "/Game/SFX/C_Bee_Death.C_Bee_Death" "0, 0, 0" "0, 0, 0" 1.0 1.0 0.0 0 0 0 0))

(event OnProjectileBounce(ProjectileMovement)
  (params (ImpactResult :type Hit%20Result%20Structure%20%28by%20ref%29) (ImpactVelocity :type Vector%20%28by%20ref%29 :default "0, 0, 0"))
  (Utilities|FlowControl|Delay 0.2)
  (Variables|/Script/Engine.ProjectileMovementComponent|SetbIsHomingProjectile (Variables|Default|GetProjectileMovement) true)
  (Variables|Default|SetWatchPlayer true)
  (Variables|/Script/Engine.ProjectileMovementComponent|SetMaxSpeed (Variables|Default|GetProjectileMovement) 6e+02)
  (Variables|Default|SetIsDashing false))

(event Custom|Dash
  (bind _projectilemovement (Variables|Default|GetProjectileMovement))
  (bind _arrow (Variables|Default|GetArrow))
  (if (not (Variables|Default|GetOff))
    (Utilities|FlowControl|Sequence
      (:then_1
        (if (<= (Math|Vector|Distance(Vector) (Transformation|GetActorLocation) (Transformation|GetActorLocation (Variables|Default|GetPlayerRef))) 2.5e+03)
          (if (not (Variables|Default|GetIsDashing))
            (Variables|/Script/Engine.ProjectileMovementComponent|SetbIsHomingProjectile _projectilemovement false)
            (Variables|/Script/Engine.MovementComponent|SetVelocity _projectilemovement "0, 0, 0")
            (Variables|Default|SetWatchPlayer false)
            (bind _predictresult (Class|GameplayStatics|BlueprintPredictProjectilePathAdvanced (Utilities|Struct|MakePredictProjectilePathParams (Transformation|GetWorldLocation _arrow) (* (Math|Vector|GetForwardVector _arrow) (Variables|Default|GetDashDistance)) true 5.0 5.0 true "ECC_WorldStatic" "ObjectTypeQuery1" (Utilities|Array|MakeArray self (Variables|Default|GetPlayerRef)) 2e+01 1.0 "ForDuration" 0.1)))
            (Utilities|FlowControl|Delay 0.5)
            (Variables|/Script/Engine.MovementComponent|SetVelocity (Variables|Default|GetProjectileMovement) (* (Math|Vector|GetForwardVector (Variables|Default|GetArrow)) 2e+03))
            (Variables|/Script/Engine.ProjectileMovementComponent|SetMaxSpeed (Variables|Default|GetProjectileMovement) (Variables|Default|GetDashSpeed))
            (Variables|Default|SetIsDashing true)
            (Utilities|Time|SetTimerbyEvent (delegate Custom|Veryfy) 2.0 true)
            (Utilities|FlowControl|DoOnce false
              (:Completed
                (if (Variables|Default|GetIsDashing)
                  (Components|Animation|PlayAnimation (Variables|Default|GetSkeletalMesh) "/Game/GameArt/Chara/A_Bee_Dash1_Anim.A_Bee_Dash1_Anim" false))))))))))

(event Custom|Veryfy
  (bind _projectilemovement (Variables|Default|GetProjectileMovement))
  (Utilities|FlowControl|Sequence
    (:then_0
      (if (Utilities|Operators|EqualEqual (.Location (Utilities|Struct|BreakPredictProjectilePathPointData (.LastTraceDestination (Utilities|Struct|BreakPredictProjectilePathResult (stale Custom|Dash _predictresult))))) (Transformation|GetActorLocation) 1e+02)
        (Variables|Default|SetIsDashing false)
        (Variables|Default|SetWatchPlayer true)
        (Variables|/Script/Engine.ProjectileMovementComponent|SetbIsHomingProjectile _projectilemovement true)
        (Variables|/Script/Engine.ProjectileMovementComponent|SetMaxSpeed _projectilemovement 4e+02)))
    (:then_1
      (Utilities|FlowControl|DoOnce false
        (:Completed
          (Components|Animation|PlayAnimation (Variables|Default|GetSkeletalMesh) "/Game/GameArt/Chara/beenoit_idlebeenoit_idle_baked_Anim.beenoit_idlebeenoit_idle_baked_Anim" true))))))

(event EventBeginPlay
  (Components|Animation|PlayAnimation (Variables|Default|GetSkeletalMesh) "/Game/GameArt/Chara/beenoit_idlebeenoit_idle_baked_Anim.beenoit_idlebeenoit_idle_baked_Anim" true)
  (bind _returnvalue (Actor|GetActorOfClass "/Game/ThirdPerson/Blueprints/BP_Player.BP_Player_C"))
  (bind _output_get (Variables|Default|SetPlayerRef _returnvalue))
  (Variables|/Script/Engine.ProjectileMovementComponent|SetHomingTargetComponent (Variables|Default|GetProjectileMovement) (Variables|/Game/ThirdPerson/Blueprints/BP_Player.BP_Player_C|GetCapsule%20bee _output_get))
  (Utilities|Time|SetTimerbyEvent (delegate Custom|Dash) 1.0 true))

(event EventTick
  (params (DeltaSeconds :type Float%20%28single-precision%29))
  (Utilities|FlowControl|Sequence
    (:then_0
      (if (not (Variables|Default|GetIsDashing))
        (Utilities|FlowControl|DoOnce false) ; enters at Reset
      ))
    (:then_1
      (if (Variables|Default|GetWatchPlayer)
        (Transformation|SetActorRotation (Math|Rotator|FindLookatRotation (Transformation|GetWorldLocation (Variables|Default|GetSphere)) (Transformation|GetActorLocation (Variables|Default|GetPlayerRef))))))))

(fn ConstructionScript)

(fn BPIProjection
  (return))