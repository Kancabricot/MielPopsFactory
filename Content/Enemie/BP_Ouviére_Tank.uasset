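; Tank worker-bee enemy that homes in on the player and takes damage from gunfire.
; On BeginPlay it loops an idle animation and targets the player's CapsuleBee with homing ProjectileMovement, while Tick keeps it facing the player.
; BP_Projectile hits on Sphere1 lower Hp; a hit at zero Hp stops homing and tracking and enables physics on the body.
; The corpse is never destroyed, and BPIProjection is empty.
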(event OnComponentHit(Sphere1)
  (params (HitComponent :type Primitive%20Component%20Object%20Reference) (OtherActor :type Actor%20Object%20Reference) (OtherComp :type Primitive%20Component%20Object%20Reference) (NormalImpulse :type Vector :default "0, 0, 0") (Hit :type Hit%20Result%20Structure%20%28by%20ref%29))
  (bind _projectilemovement (Variables|Default|GetProjectileMovement))
  (Utilities|Casting|CastToBP_Projectile OtherActor)
  (Audio|PlaySoundatLocation "/Game/SFX/C_Impact_Gun.C_Impact_Gun" "0, 0, 0" "0, 0, 0" 0.6 1.0 0.0 0 0 0 0)
  (if (not (<= (Variables|Default|GetHp) 0.0))
    (Variables|Default|SetHp (- (Variables|Default|GetHp) 1e+01))
    (else
      (Physics|SetSimulatePhysics (Variables|Default|GetSphere) true)
      (Physics|SetSimulatePhysics (Variables|Default|GetSkeletalMesh) true)
      (Audio|Components|Audio|Stop (Variables|Default|GetSkeletalMesh))
      (Variables|/Script/Engine.ProjectileMovementComponent|SetbShouldBounce _projectilemovement false)
      (Variables|/Script/Engine.ProjectileMovementComponent|SetbIsHomingProjectile _projectilemovement false)
      (Variables|Default|SetWatchPlayer false))))

(event EventBeginPlay
  (Components|Animation|PlayAnimation (Variables|Default|GetSkeletalMesh) "/Game/GameArt/Chara/beenoit_idlebeenoit_idle_baked_Anim.beenoit_idlebeenoit_idle_baked_Anim" true)
  (bind _returnvalue (Actor|GetActorOfClass "/Game/ThirdPerson/Blueprints/BP_Player.BP_Player_C"))
  (bind _output_get (Variables|Default|SetPlayerRef _returnvalue))
  (Variables|/Script/Engine.ProjectileMovementComponent|SetHomingTargetComponent (Variables|Default|GetProjectileMovement) (Variables|/Game/ThirdPerson/Blueprints/BP_Player.BP_Player_C|GetCapsule%20bee _output_get)))

(event EventTick
  (params (DeltaSeconds :type Float%20%28single-precision%29))
  (if (Variables|Default|GetWatchPlayer)
    (Transformation|SetActorRotation (Math|Rotator|FindLookatRotation (Transformation|GetWorldLocation (Variables|Default|GetSphere)) (Transformation|GetActorLocation (Variables|Default|GetPlayerRef))))))

(fn ConstructionScript)

(fn BPIProjection
  (return))