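; BP_Spawner is a trigger-based enemy spawner that spawns a configurable actor class when its box is overlapped.
; An overlap optionally shows an Event_Warn widget and, if the spawner is active, starts a looping timer.
; Each tick of that timer spawns a scaled-up actor at the spawner's transform until the spawn counter reaches the enemy limit.
; The overlap has no filter on the overlapping actor or guard against retriggering.
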(event OnComponentBeginOverlap(Box)
  (params (OverlappedComponent :type Primitive%20Component%20Object%20Reference) (OtherActor :type Actor%20Object%20Reference) (OtherComp :type Primitive%20Component%20Object%20Reference) (OtherBodyIndex :type Integer) (bFromSweep :type Boolean) (SweepResult :type Hit%20Result%20Structure%20%28by%20ref%29))
  (if (Variables|Default|GetShowMessage)
    (bind _returnvalue (UserInterface|CreateWidget "/Game/Enemie/Event_Warn.Event_Warn_C" (Game|GetPlayerController 0)))
    (UserInterface|Viewport|AddtoViewport _returnvalue 0))
  (if (Variables|Default|GetACTIVE)
    (Utilities|Time|SetTimerbyEvent (delegate Custom|Spawn) 2.0 true)))

(event Custom|Spawn
  (bind _returnvalue (Transformation|GetActorTransform))
  (if (not (>= (Variables|Default|GetEnemySpawn) (Variables|Default|GetNbEnemy)))
    (Game|SpawnActorfromClass (Variables|Default|GetActorToSpawn) (Math|Transform|MakeTransform (.location _returnvalue) (.rotation _returnvalue) "5.000000,5.000000,5.000000") "Undefined" 0 0)
    (Variables|Default|SetEnemySpawn (+ (Variables|Default|GetEnemySpawn) 1))))

(event EventBeginPlay)

(event Collision|EventActorBeginOverlap
  (params (OtherActor :type Actor%20Object%20Reference)))

(fn ConstructionScript)