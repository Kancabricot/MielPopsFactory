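; BP_Queen is an enemy that pursues the player through projectile-movement homing and performs a telegraphed straight-line dash.
; While WatchPlayer is set, Tick rotates it toward the player.
; When the player enters DetectionZone, it stops, briefly draws a predicted path along its arrow, waits, then launches forward.
; A looping timer compares its location with the predicted endpoint and restores homing, facing and slower speed on arrival.
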(event OnComponentBeginOverlap(DetectionZone)
  (params (OverlappedComponent :type Primitive%20Component%20Object%20Reference) (OtherActor :type Actor%20Object%20Reference) (OtherComp :type Primitive%20Component%20Object%20Reference) (OtherBodyIndex :type Integer) (bFromSweep :type Boolean) (SweepResult :type Hit%20Result%20Structure%20%28by%20ref%29))
  (bind _projectilemovement (Variables|Default|GetProjectileMovement))
  (bind _arrow (Variables|Default|GetArrow))
  (Utilities|Casting|CastToBP_ThirdPersonCharacter OtherActor)
  (if (not (Variables|Default|GetIsDashing))
    (Variables|/Script/Engine.ProjectileMovementComponent|SetbIsHomingProjectile _projectilemovement false)
    (Variables|/Script/Engine.MovementComponent|SetVelocity _projectilemovement "0, 0, 0")
    (Variables|Default|SetWatchPlayer false)
    (bind _predictresult (Class|GameplayStatics|BlueprintPredictProjectilePathAdvanced (Utilities|Struct|MakePredictProjectilePathParams (Transformation|GetWorldLocation _arrow) (* (Math|Vector|GetForwardVector _arrow) (Variables|Default|GetDashDistance)) true 5.0 5.0 true "ECC_WorldStatic" "ObjectTypeQuery1" (Utilities|Array|MakeArray self (Variables|Default|GetPlayerRef)) 2e+01 1.0 "ForDuration" 0.1)))
    (Utilities|FlowControl|Delay 1.0)
    (Variables|/Script/Engine.MovementComponent|SetVelocity (Variables|Default|GetProjectileMovement) (* (Math|Vector|GetForwardVector (Variables|Default|GetArrow)) 1e+03))
    (Variables|/Script/Engine.ProjectileMovementComponent|SetMaxSpeed (Variables|Default|GetProjectileMovement) (Variables|Default|GetDashSpeed))
    (Variables|Default|SetIsDashing true)
    (Utilities|Time|SetTimerbyEvent (delegate Custom|Veryfy) 0.1 true)))

(event OnComponentHit(Sphere)
  (params (HitComponent :type Primitive%20Component%20Object%20Reference) (OtherActor :type Actor%20Object%20Reference) (OtherComp :type Primitive%20Component%20Object%20Reference) (NormalImpulse :type Vector :default "0, 0, 0") (Hit :type Hit%20Result%20Structure%20%28by%20ref%29)))

(event Custom|Veryfy
  (bind _projectilemovement (Variables|Default|GetProjectileMovement))
  (if (Utilities|Operators|EqualEqual (.Location (Utilities|Struct|BreakPredictProjectilePathPointData (.LastTraceDestination (Utilities|Struct|BreakPredictProjectilePathResult (stale OnComponentBeginOverlap(DetectionZone) _predictresult))))) (Transformation|GetActorLocation) 1e+02)
    (Variables|Default|SetIsDashing false)
    (Variables|Default|SetWatchPlayer true)
    (Variables|/Script/Engine.ProjectileMovementComponent|SetbIsHomingProjectile _projectilemovement true)
    (Variables|/Script/Engine.ProjectileMovementComponent|SetMaxSpeed _projectilemovement 4e+02)))

(event EventBeginPlay
  (bind _returnvalue (Actor|GetActorOfClass "/Game/ThirdPerson/Blueprints/BP_ThirdPersonCharacter.BP_ThirdPersonCharacter_C"))
  (bind _output_get (Variables|Default|SetPlayerRef _returnvalue))
  (Variables|/Script/Engine.ProjectileMovementComponent|SetHomingTargetComponent (Variables|Default|GetProjectileMovement) (Variables|/Script/Engine.Character|GetCapsuleComponent _output_get)))

(event EventTick
  (params (DeltaSeconds :type Float%20%28single-precision%29))
  (if (Variables|Default|GetWatchPlayer)
    (Transformation|SetActorRotation (Math|Rotator|FindLookatRotation (Transformation|GetWorldLocation (Variables|Default|GetSphere)) (Transformation|GetActorLocation (Variables|Default|GetPlayerRef))))))

(fn ConstructionScript)