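; BP_Ouviére_Tireuse_2 is an enemy-folder actor that homes in on the player through its ProjectileMovement component.
; On BeginPlay it finds BP_Player and sets that actor's CapsuleBee as the homing target.
; Each tick, while WatchPlayer is set, it rotates from its Sphere's location to face the player.
; Sphere hits only print a debug string, and the BPI_Projection function is an empty stub.
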(event OnComponentHit(Sphere)
  (params (HitComponent :type Primitive%20Component%20Object%20Reference) (OtherActor :type Actor%20Object%20Reference) (OtherComp :type Primitive%20Component%20Object%20Reference) (NormalImpulse :type Vector :default "0, 0, 0") (Hit :type Hit%20Result%20Structure%20%28by%20ref%29))
  (Development|PrintString "Hello"))

(event EventBeginPlay
  (bind _returnvalue (Actor|GetActorOfClass "/Game/ThirdPerson/Blueprints/BP_Player.BP_Player_C"))
  (bind _output_get (Variables|Default|SetPlayerRef _returnvalue))
  (Variables|/Script/Engine.ProjectileMovementComponent|SetHomingTargetComponent (Variables|Default|GetProjectileMovement) (Variables|/Game/ThirdPerson/Blueprints/BP_Player.BP_Player_C|GetCapsule%20bee _output_get)))

(event EventTick
  (params (DeltaSeconds :type Float%20%28single-precision%29))
  (if (Variables|Default|GetWatchPlayer)
    (Transformation|SetActorRotation (Math|Rotator|FindLookatRotation (Transformation|GetWorldLocation (Variables|Default|GetSphere)) (Transformation|GetActorLocation (Variables|Default|GetPlayerRef))))))

(fn ConstructionScript)

(fn BPIProjection
  (return))