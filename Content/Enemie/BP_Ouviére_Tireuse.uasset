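; Shooter worker enemy that chases the player using a homing ProjectileMovement component and can rotate to face them.
; When the player enters DetectionZone, it stops homing and a looping timer spawns projectiles while alternating random positive and negative velocity drifts.
; Leaving the zone pauses firing and resumes the chase.
; A BP_Projectile overlapping its Sphere launches it along the shot's direction, adds a Niagara component and destroys that projectile.
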(event OnComponentBeginOverlap(DetectionZone)
  (params (OverlappedComponent :type Primitive%20Component%20Object%20Reference) (OtherActor :type Actor%20Object%20Reference) (OtherComp :type Primitive%20Component%20Object%20Reference) (OtherBodyIndex :type Integer) (bFromSweep :type Boolean) (SweepResult :type Hit%20Result%20Structure%20%28by%20ref%29))
  (bind _projectilemovement (Variables|Default|GetProjectileMovement))
  (Utilities|Casting|CastToBP_Player OtherActor)
  (Variables|/Script/Engine.ProjectileMovementComponent|SetbIsHomingProjectile _projectilemovement false)
  (Variables|/Script/Engine.MovementComponent|SetVelocity _projectilemovement "0, 0, 0")
  (bind _returnvalue (Utilities|Time|SetTimerbyEvent (delegate Custom|Shoot) 1.0 true))
  (Variables|Default|SetShootTimer _returnvalue))

(event OnComponentEndOverlap(DetectionZone)
  (params (OverlappedComponent :type Primitive%20Component%20Object%20Reference) (OtherActor :type Actor%20Object%20Reference) (OtherComp :type Primitive%20Component%20Object%20Reference) (OtherBodyIndex :type Integer))
  (bind _projectilemovement (Variables|Default|GetProjectileMovement))
  (Utilities|Casting|CastToBP_Player OtherActor)
  (Variables|/Script/Engine.ProjectileMovementComponent|SetbIsHomingProjectile _projectilemovement true)
  (Variables|/Script/Engine.MovementComponent|SetVelocity _projectilemovement (* (Math|Vector|GetForwardVector (Variables|Default|GetArrow)) 2e+03))
  (Variables|/Script/Engine.ProjectileMovementComponent|SetMaxSpeed _projectilemovement 4e+02)
  (Utilities|Time|PauseTimerbyHandle (Variables|Default|GetShootTimer)))

(event OnComponentBeginOverlap(Sphere)
  (params (OverlappedComponent :type Primitive%20Component%20Object%20Reference) (OtherActor :type Actor%20Object%20Reference) (OtherComp :type Primitive%20Component%20Object%20Reference) (OtherBodyIndex :type Integer) (bFromSweep :type Boolean) (SweepResult :type Hit%20Result%20Structure%20%28by%20ref%29))
  (bind _projectilemovement (Variables|Default|GetProjectileMovement))
  (bind _asbp_projectile (Utilities|Casting|CastToBP_Projectile OtherActor))
  (Variables|/Script/Engine.ProjectileMovementComponent|SetbIsHomingProjectile _projectilemovement false)
  (Variables|/Script/Engine.ProjectileMovementComponent|SetbShouldBounce _projectilemovement false)
  (Variables|/Script/Engine.ProjectileMovementComponent|SetMaxSpeed _projectilemovement 3e+03)
  (Variables|/Script/Engine.MovementComponent|SetVelocity _projectilemovement (* (Math|Vector|GetForwardVector (Variables|/Game/Projectile/BP_Projectile.BP_Projectile_C|GetArrow _asbp_projectile)) 3e+03))
  (AddComponent|AddNiagaraComponent false (Transformation|GetRelativeTransform (Variables|Default|GetCube)))
  (Actor|DestroyActor _asbp_projectile))

(event OnComponentHit(Sphere)
  (params (HitComponent :type Primitive%20Component%20Object%20Reference) (OtherActor :type Actor%20Object%20Reference) (OtherComp :type Primitive%20Component%20Object%20Reference) (NormalImpulse :type Vector :default "0, 0, 0") (Hit :type Hit%20Result%20Structure%20%28by%20ref%29))
  (Development|PrintString "Hello"))

(event Custom|Shoot
  (bind _returnvalue (Math|Random|RandomFloatinRange 1e+02 1.5e+02))
  (bind _projectilemovement (Variables|Default|GetProjectileMovement))
  (bind _returnvalue_2 (* _returnvalue -1.0))
  (Variables|Default|SetRandPoint (Math|Random|RandomInteger 5))
  (Game|SpawnActorfromClass "/Game/Enemie/Projo/Bp_ProjoOuvriére.Bp_ProjoOuvriére_C" (Transformation|GetActorTransform) "AdjustIfPossibleButAlwaysSpawn" 0 0)
  (Variables|/Script/Engine.ProjectileMovementComponent|SetMaxSpeed _projectilemovement 4e+02)
  (Utilities|FlowControl|FlipFlop
    (:A
      (Variables|/Script/Engine.MovementComponent|SetVelocity _projectilemovement (Math|Vector|MakeVector _returnvalue _returnvalue _returnvalue)))
    (:B
      (Variables|/Script/Engine.MovementComponent|SetVelocity _projectilemovement (Math|Vector|MakeVector _returnvalue_2 _returnvalue_2 _returnvalue_2)))))

(event EventBeginPlay
  (bind _returnvalue (Actor|GetActorOfClass "/Game/ThirdPerson/Blueprints/BP_Player.BP_Player_C"))
  (bind _output_get (Variables|Default|SetPlayerRef _returnvalue))
  (Variables|/Script/Engine.ProjectileMovementComponent|SetHomingTargetComponent (Variables|Default|GetProjectileMovement) (Variables|/Game/ThirdPerson/Blueprints/BP_Player.BP_Player_C|GetCapsule%20bee _output_get)))

(event EventTick
  (params (DeltaSeconds :type Float%20%28single-precision%29))
  (if (Variables|Default|GetWatchPlayer)
    (Transformation|SetActorRotation (Math|Rotator|FindLookatRotation (Transformation|GetWorldLocation (Variables|Default|GetSphere)) (Transformation|GetActorLocation (Variables|Default|GetPlayerRef))))))

(fn ConstructionScript)

(fn BPIProjection
  (return))