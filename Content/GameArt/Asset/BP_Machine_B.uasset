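; BP_Machine_B is a destructible machine with four hit zones that counts toward a quest and can unlock a door.
; Each zone overlapped by a BP_Projectile is removed from the tracking array, destroyed and added to a counter.
; Once the counter reaches NumberOfDestroy, the machine notifies its linked door, destroys itself with explosion sound and Niagara effect, and calls AddQuest1 on the supplied quest widget reference.
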(event OnComponentBeginOverlap(DestroyZone2)
  (params (OverlappedComponent :type Primitive%20Component%20Object%20Reference) (OtherActor :type Actor%20Object%20Reference) (OtherComp :type Primitive%20Component%20Object%20Reference) (OtherBodyIndex :type Integer) (bFromSweep :type Boolean) (SweepResult :type Hit%20Result%20Structure%20%28by%20ref%29))
  (bind _destroy_zone2 (Variables|Default|GetDestroy%20Zone2))
  (Utilities|Casting|CastToBP_Projectile OtherActor)
  (Utilities|Array|RemoveItem (Variables|Default|GetArrayOfZoneToDestroy) _destroy_zone2)
  (Components|DestroyComponent _destroy_zone2)
  (Variables|Default|SetNumberOfObjectDestroy (+ (Variables|Default|GetNumberOfObjectDestroy) 1))
  (CallFunction|CheckDestroyFacory))

(event OnComponentBeginOverlap(DestroyZone3)
  (params (OverlappedComponent :type Primitive%20Component%20Object%20Reference) (OtherActor :type Actor%20Object%20Reference) (OtherComp :type Primitive%20Component%20Object%20Reference) (OtherBodyIndex :type Integer) (bFromSweep :type Boolean) (SweepResult :type Hit%20Result%20Structure%20%28by%20ref%29))
  (bind _destroy_zone3 (Variables|Default|GetDestroy%20Zone3))
  (Utilities|Casting|CastToBP_Projectile OtherActor)
  (Utilities|Array|RemoveItem (Variables|Default|GetArrayOfZoneToDestroy) _destroy_zone3)
  (Components|DestroyComponent _destroy_zone3)
  (Variables|Default|SetNumberOfObjectDestroy (+ (Variables|Default|GetNumberOfObjectDestroy) 1))
  (CallFunction|CheckDestroyFacory))

(event OnComponentBeginOverlap(DestroyZone4)
  (params (OverlappedComponent :type Primitive%20Component%20Object%20Reference) (OtherActor :type Actor%20Object%20Reference) (OtherComp :type Primitive%20Component%20Object%20Reference) (OtherBodyIndex :type Integer) (bFromSweep :type Boolean) (SweepResult :type Hit%20Result%20Structure%20%28by%20ref%29))
  (bind _destroy_zone4 (Variables|Default|GetDestroy%20Zone4))
  (Utilities|Casting|CastToBP_Projectile OtherActor)
  (Utilities|Array|RemoveItem (Variables|Default|GetArrayOfZoneToDestroy) _destroy_zone4)
  (Components|DestroyComponent _destroy_zone4)
  (Variables|Default|SetNumberOfObjectDestroy (+ (Variables|Default|GetNumberOfObjectDestroy) 1))
  (CallFunction|CheckDestroyFacory))

(event OnComponentBeginOverlap(DestroyZone1)
  (params (OverlappedComponent :type Primitive%20Component%20Object%20Reference) (OtherActor :type Actor%20Object%20Reference) (OtherComp :type Primitive%20Component%20Object%20Reference) (OtherBodyIndex :type Integer) (bFromSweep :type Boolean) (SweepResult :type Hit%20Result%20Structure%20%28by%20ref%29))
  (bind _destroy_zone1 (Variables|Default|GetDestroy%20Zone1))
  (Utilities|Casting|CastToBP_Projectile OtherActor)
  (Utilities|Array|RemoveItem (Variables|Default|GetArrayOfZoneToDestroy) _destroy_zone1)
  (Components|DestroyComponent _destroy_zone1)
  (Variables|Default|SetNumberOfObjectDestroy (+ (Variables|Default|GetNumberOfObjectDestroy) 1))
  (CallFunction|CheckDestroyFacory))

(event Custom|Getref
  (params (QuestWGRef :type WG%20Quest%20Object%20Reference))
  (Variables|Default|SetQuestWGRef QuestWGRef))

(event EventBeginPlay
  (Utilities|Array|Add (Variables|Default|GetArrayOfZoneToDestroy) (Variables|Default|GetDestroy%20Zone1))
  (Utilities|Array|Add (Variables|Default|GetArrayOfZoneToDestroy) (Variables|Default|GetDestroy%20Zone2))
  (Utilities|Array|Add (Variables|Default|GetArrayOfZoneToDestroy) (Variables|Default|GetDestroy%20Zone3))
  (Utilities|Array|Add (Variables|Default|GetArrayOfZoneToDestroy) (Variables|Default|GetDestroy%20Zone4)))

(fn ConstructionScript)

(fn CheckDestroyFacory
  (bind _returnvalue (Transformation|GetActorLocation))
  (if (>= (Variables|Default|GetNumberOfObjectDestroy) (Variables|Default|GetNumberOfDestroy))
    (bind _doortounlock (Variables|Default|GetDoorToUnlock)
      (:then
        (Default|ChecktoUnlockDoor _doortounlock))
      (:else
        _))
    (Actor|DestroyActor)
    (Audio|PlaySoundatLocation "/Game/SFX/C_Machine_Explo.C_Machine_Explo" _returnvalue "0, 0, 0" 1.0 1.0 0.0 0 0 0 0)
    (Niagara|SpawnSystematLocation "/Game/VFX/Stylized_Explosion/NS_Explosion.NS_Explosion" _returnvalue "0, 0, 0" "1.500000,1.500000,1.500000")
    (Default|AddQuest1 (Variables|Default|GetQuestWGRef))))